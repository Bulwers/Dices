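; Board spot actor that highlights when the cursor hovers over it as a potential target for a dice buff.
; It hides its Plane and enables player-controller mouse-over events on BeginPlay.
; Hovering shows the Plane only with the camera in Top position, a plus-one or plus-two buff active and valid player dice in its TriggerArea.
; A timeline drives the material opacity, and cursor exit hides the Plane under the same conditions.
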(event `self.ReceiveBeginPlay`
  (`SceneComponent.SetVisibility` (`self.Plane`) false false)
  (set `PlayerController.bEnableMouseOverEvents` true (`GameplayStatics.GetPlayerController` 0)))

(event `self.ReceiveActorBeginCursorOver`
  (bind _plane (`self.Plane`))
  (bind _player (`self.Player`))
  (if (and (`|EnumEquality` (`PlayerCameraManagerComponent.GetCurrentCamPos` (`BasePlayer.CameraComp` _player)) "Top") (or (`BasePlayer.bPlusOneBuff` _player) (`BasePlayer.bPlusTwoBuff` _player)) (`KismetSystemLibrary.IsValid` (`BuffTriggerAreaComponent.PlayerDice` (`self.TriggerArea`))))
    (`SceneComponent.SetVisibility` _plane true false)
    (bind (_direction _alpha) (`Timeline|Timeline` :`NewTime` 4.0 :!via `PlayFromStart` :!label _label)
      (:`Update`
        (`MeshComponent.SetScalarParameterValueOnMaterials` _plane "Opacity" (`KismetMathLibrary.Lerp` 0.0 0.3 _alpha))))))

(event `self.ReceiveActorEndCursorOver`
  (bind _player (`self.Player`))
  (if (and (`|EnumEquality` (`PlayerCameraManagerComponent.GetCurrentCamPos` (`BasePlayer.CameraComp` _player)) "Top") (or (`BasePlayer.bPlusOneBuff` _player) (`BasePlayer.bPlusTwoBuff` _player)) (`KismetSystemLibrary.IsValid` (`BuffTriggerAreaComponent.PlayerDice` (`self.TriggerArea`))))
    (`SceneComponent.SetVisibility` (`self.Plane`) false false)
    (goto _label :!via `Stop`)))

(fn `UserConstructionScript`)