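; BP_FakeDice is a dice actor that highlights its mesh when the cursor hovers over it.
; BeginPlay enables mouse-over events, and hovering applies the highlight material to a highlightable player die unless it is chosen but not yet rolled.
; Cursor exit restores the normal material on player dice, while Tick calls SetMaterial to keep chosen, unrolled dice on that material.
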(event `self.ReceiveBeginPlay`
  (set `PlayerController.bEnableMouseOverEvents` true (`GameplayStatics.GetPlayerController` 0)))

(event `self.ReceiveActorBeginCursorOver`
  (if (and (`self.bIsPlayer`) (`self.bCanHighlight`))
    (if (`self.bIsChoosen`)
      (if (`self.bIsRolled`)
        (`PrimitiveComponent.SetMaterial` (`self.DiceMesh`) 0 "/Game/Dynamic/Dices/HighlightMaterial.HighlightMaterial" :!label _label))
      (else
        (goto _label)))))

(event `self.ReceiveActorEndCursorOver`
  (if (`self.bIsPlayer`)
    (`PrimitiveComponent.SetMaterial` (`self.DiceMesh`) 0 "/Game/Dynamic/Dices/Material.Material")))

(event `self.ReceiveTick`
  (params (DeltaSeconds :type "Float (single-precision)"))
  (`self.SetMaterial`))

(fn `SetMaterial`
  (if (`self.bIsChoosen`)
    (if (not (`self.bIsRolled`))
      (`PrimitiveComponent.SetMaterial` (`self.DiceMesh`) 0 "/Game/Dynamic/Dices/Material.Material"))))

(fn `UserConstructionScript`)